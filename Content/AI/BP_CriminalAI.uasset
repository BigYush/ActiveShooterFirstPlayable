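; BP_CriminalAI is an AI controller for a criminal NPC, but its possess and perception events are empty, so it currently does nothing.
; Disconnected logic would run BT_CriminalAI and loop perceived actors' stimuli, treating array index 0 as sight and 1 as noise.
; That logic would write CanSeePlayer, ShouldInvesigate (misspelled) and InvestigateLocation to the Blackboard, with debug prints throughout.
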(event OnPerceptionUpdated(AIPerception)
  (params (UpdatedActors :type Array%20of%20Actor%20Object%20References)))

(event EventBeginPlay)

(event EventPossess
  (params (PossessedPawn :type Pawn%20Object%20Reference)))

(fn ConstructionScript)